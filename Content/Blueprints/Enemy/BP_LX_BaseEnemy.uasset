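; Base enemy that spots the player through AI perception, turns to face them and fires light-ball projectiles.
; Perception pauses or resumes a looping shoot timer, whose attack animation triggers left and right projectile spawns that damage what they hit.
; A damage component drives death, block, parry and hit responses.
; It can also be grabbed with damped physics, and slashes deal damage scaled by impulse.
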(event `self.ReceiveBeginPlay`
  (bind _returnvalue (`KismetSystemLibrary.K2_SetTimer` null "ShootPlayer" (`self.ShootDelay`) true false 0.0 0.5))
  (set `self.ShootTimerHandle` _returnvalue)
  (`KismetSystemLibrary.K2_PauseTimer` null "ShootPlayer"))

(event `SpawnRightProjectile`
  (bind _returnvalue (`|SpawnActorFromClass` "/Game/Blueprints/Enemy/BP_LX_LightBall.BP_LX_LightBall_C" (`SceneComponent.K2_GetComponentToWorld` (`self.RightProjSpawnPoint`)) "Undefined" "MultiplyWithRoot" self (`self.ProjectileSpeed`) (`self.CurrentTrackedPawn`) null))
  (add `/Game/Blueprints/Enemy/BP_LX_BaseProjectile.OnProjectileHit` _returnvalue (`|CreateDelegate` :!event `RightDamagePlayer`))
  (`GameplayStatics.PlaySoundAtLocation` "/Game/Blueprints/Enemy/SW_EnemyAttackBurst.SW_EnemyAttackBurst" (`self.K2_GetActorLocation`) (struct) 1.0 1.0 0.0 null null null null))

(event `self.ReceiveTick`
  (params (DeltaSeconds :type "Float (single-precision)"))
  (bind (_returnvalue_roll _returnvalue_pitch _returnvalue_yaw) (`KismetMathLibrary.BreakRotator` (`KismetMathLibrary.RLerp` (`KismetMathLibrary.FindLookAtRotation` (`self.K2_GetActorLocation`) (`self.K2_GetActorLocation` (`self.CurrentTrackedPawn`))) (`self.K2_GetActorRotation`) DeltaSeconds)))
  ; Rotate to target if a target is being tracked
  (if (`self.IsTracking`)
    (`SceneComponent.K2_SetWorldRotation` (`self.Scene`) (`KismetMathLibrary.MakeRotator` 0.0 _returnvalue_pitch _returnvalue_yaw) false false)))

(event `SpawnLeftProjectile`
  (bind _returnvalue (`|SpawnActorFromClass` "/Game/Blueprints/Enemy/BP_LX_LightBall.BP_LX_LightBall_C" (`SceneComponent.K2_GetComponentToWorld` (`self.LeftProjSpawnPoint`)) "Undefined" "MultiplyWithRoot" self (`self.ProjectileSpeed`) (`self.CurrentTrackedPawn`) null))
  (add `/Game/Blueprints/Enemy/BP_LX_BaseProjectile.OnProjectileHit` _returnvalue (`|CreateDelegate` :!event `LeftDamagePlayer`))
  (`GameplayStatics.PlaySoundAtLocation` "/Game/Blueprints/Enemy/SW_EnemyAttackBurst.SW_EnemyAttackBurst" (`self.K2_GetActorLocation`) (struct) 1.0 1.0 0.0 null null null null))

(event `self.AIPerception.OnTargetPerceptionUpdated`
  (params (Actor :type "Actor Object Reference") (Stimulus :type "AIStimulus Structure"))
  (bind _returnvalue (`GameplayStatics.GetPlayerPawn` 0))
  ; Track pawn
  (if (`/Game/DamageSystem/BPC_LX_DamageComponent.IsDead` (`self.BPC_LX_DamageComponent`))
    _
    (elif (== Actor _returnvalue)
      (bind _output_get (set `self.IsTracking` (`.bSuccessfullySensed` (break `AIStimulus` Stimulus))))
      (if _output_get
        (set `self.CurrentTrackedPawn` _returnvalue)
        (`KismetSystemLibrary.K2_UnPauseTimer` null "ShootPlayer")
        ; Set animation for player sensed and ready to attack
        (`SkeletalMeshComponent.SetAnimation` (`self.SkeletalMesh`) "/Game/ElfArden/Animations/AS_idle.AS_idle")
        (`SkeletalMeshComponent.Play` (`self.SkeletalMesh`) true)
        (`GameplayStatics.PlaySoundAtLocation` "/Game/Blueprints/Enemy/SW_PlayerSpottedGrunt.SW_PlayerSpottedGrunt" (`self.K2_GetActorLocation`) (struct) 1.0 1.0 0.0 null null null null)
        (else
          (`KismetSystemLibrary.K2_PauseTimer` null "ShootPlayer")
          (`SkeletalMeshComponent.SetAnimation` (`self.SkeletalMesh`) "/Game/ElfArden/Animations/EpicSkeleton_UE5/AS_Idle.AS_Idle")
          (`SkeletalMeshComponent.Play` (`self.SkeletalMesh`) true))))))

(event `Death`
  (`KismetSystemLibrary.PrintString` "enemy death")
  (`KismetSystemLibrary.K2_ClearAndInvalidateTimerHandle` (`self.ShootTimerHandle`))
  (`SkeletalMeshComponent.SetAnimation` (`self.SkeletalMesh`) "/Game/Blueprints/Enemy/Animations/AS_deadwnotify.AS_deadwnotify")
  (`SkeletalMeshComponent.Play` (`self.SkeletalMesh`) false)
  (`GameplayStatics.PlaySoundAtLocation` "/Game/Blueprints/Sword/kill.kill" (`self.K2_GetActorLocation`) (struct) 1.0 1.0 0.0 null null null null)
  (`PrimitiveComponent.SetCollisionResponseToChannel` (`self.SkeletalMesh`) "ECC_GameTraceChannel1" "ECR_Block"))

(event `Block`
  (`KismetSystemLibrary.PrintString` "blocked on enemy"))

(event `Parry`
  (`KismetSystemLibrary.PrintString` "parried on enemy"))

(event `DamageResponse`
  (params (DamageResponse :type "/Game/DamageSystem/E_LX_DamageResponse Enum" :default "NewEnumerator0"))
  (`KismetSystemLibrary.PrintString` (`|GetEnumeratorNameAsString` DamageResponse))
  (`GameplayStatics.PlaySoundAtLocation` "/Game/Blueprints/Enemy/SW_AttackedGrunt.SW_AttackedGrunt" (`self.K2_GetActorLocation`) (struct) 1.0 1.0 0.0 null null null null))

(event `RightDamagePlayer`
  (params (OtherActor :type "/Game/DamageSystem/BPC_LX_DamageComponent Object Reference") (DamageInfo :type "/Game/DamageSystem/S_LX_DamageInfo Structure") (Hit :type "HitResult Structure"))
  (`/Game/DamageSystem/BPC_LX_DamageComponent.TakeDamage` OtherActor DamageInfo))

(event `LeftDamagePlayer`
  (params (OtherActor :type "/Game/DamageSystem/BPC_LX_DamageComponent Object Reference") (DamageInfo :type "/Game/DamageSystem/S_LX_DamageInfo Structure") (Hit :type "HitResult Structure"))
  (`/Game/DamageSystem/BPC_LX_DamageComponent.TakeDamage` OtherActor DamageInfo))

(event `/Game/BlueprintInterface/BPI_Interaction.InteractBegin`
  (params (Player :type "/Game/Blueprints/VRPawn Object Reference"))
  (bind _skeletalmeshroot (`self.SkeletalMeshRoot`))
  ; Grab
  (`PrimitiveComponent.SetSimulatePhysics` _skeletalmeshroot true)
  (`PrimitiveComponent.SetLinearDamping` _skeletalmeshroot 25.0))

(event `/Game/BlueprintInterface/BPI_Interaction.InteractEnd`
  (params (Player :type "/Game/Blueprints/VRPawn Object Reference"))
  (bind _skeletalmeshroot (`self.SkeletalMeshRoot`))
  ; Grab
  (`PrimitiveComponent.SetSimulatePhysics` _skeletalmeshroot false)
  (`PrimitiveComponent.SetLinearDamping` _skeletalmeshroot 0.01))

(event `/Game/BlueprintInterface/BPI_Slashable.Slash`
  (params (Impulse :type "Vector Structure"))
  (bind _wasdamaged (`/Game/DamageSystem/BPC_LX_DamageComponent.TakeDamage` (`self.BPC_LX_DamageComponent`) (make `/Game/DamageSystem/S_LX_DamageInfo` (/ (`KismetMathLibrary.VSize` Impulse) 1000.0) "NewEnumerator1")))
  (if _wasdamaged
    (`GameplayStatics.PlaySoundAtLocation` "/Game/Blueprints/Sword/slice.slice" (`self.K2_GetActorLocation`) (struct) 1.0 1.0 0.0 null null null null)))

(event `/Game/BlueprintInterface/BPI_Overlappable.Overlap`
  (params (ImpactPoint :type "Vector Structure"))
  (`GameplayStatics.SpawnEmitterAtLocation` "/Game/Blueprints/Sword/P_Blood.P_Blood" ImpactPoint))

(fn `GetActor`
  (returns (Actor :type "Actor Object Reference"))
  (return null))

(fn `ShootPlayer`
  (`SkeletalMeshComponent.SetAnimation` (`self.SkeletalMesh`) "/Game/Blueprints/Enemy/Animations/AS_attackwnotify.AS_attackwnotify")
  (`SkeletalMeshComponent.Play` (`self.SkeletalMesh`) false)
  (add `self.OnSpawnRightProjectile` (`|CreateDelegate` :!event `SpawnRightProjectile`))
  (add `self.OnSpawnLeftProjectile` (`|CreateDelegate` :!event `SpawnLeftProjectile`)))

(fn `TakeDamage`
  (params (DamageInfo :type "/Game/DamageSystem/S_LX_DamageInfo Structure"))
  (returns (WasDamaged :type Boolean))
  (bind _wasdamaged (`/Game/DamageSystem/BPI_LX_Damagable.TakeDamage` (`self.BPC_LX_DamageComponent`) DamageInfo))
  (return _wasdamaged))

(fn `UserConstructionScript`
  (add `/Game/DamageSystem/BPC_LX_DamageComponent.OnDeath` (`self.BPC_LX_DamageComponent`) (`|CreateDelegate` :!event `Death`))
  (add `/Game/DamageSystem/BPC_LX_DamageComponent.OnBlock` (`self.BPC_LX_DamageComponent`) (`|CreateDelegate` :!event `Block`))
  (add `/Game/DamageSystem/BPC_LX_DamageComponent.OnParry` (`self.BPC_LX_DamageComponent`) (`|CreateDelegate` :!event `Parry`))
  (add `/Game/DamageSystem/BPC_LX_DamageComponent.OnDamageResponse` (`self.BPC_LX_DamageComponent`) (`|CreateDelegate` :!event `DamageResponse`)))