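; TimeSlowZone is an actor that slows global time to SlowFactor alongside a post-process colour effect and clock-ticking sound.
; On BeginPlay, the ColourChange timeline drives BW_Amount on a dynamic post-process material, re-triggering the sound and slowdown every update.
; Tick destroys the actor once BW_Amount reaches zero, without restoring time.
; The Destroyer event stops the sound, destroys the actor and restores normal time.
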(event `self.ReceiveTick`
  (params (DeltaSeconds :type "Float (single-precision)"))
  (bind _returnvalue (`MaterialInstanceDynamic.K2_GetScalarParameterValue` (`self.DynamicPPMaterial`) "BW_Amount"))
  (if (<= _returnvalue 0.0)
    (`self.K2_DestroyActor`)))

(event `self.ReceiveBeginPlay`
  (bind _returnvalue (`KismetMaterialLibrary.CreateDynamicMaterialInstance` "/Game/Blueprints/TimeSlow/PostProcessMaterial.PostProcessMaterial"))
  (set `self.DynamicPPMaterial` _returnvalue)
  (bind (_direction _bwtonormal) (`Timeline|ColourChange`)
    (:`Update`
      (`PostProcessComponent.AddOrUpdateBlendable` (`self.PostProcess`) (`self.DynamicPPMaterial`) 1.0)
      (`MaterialInstanceDynamic.SetScalarParameterValue` (`self.DynamicPPMaterial`) "BW_Amount" _bwtonormal)
      (`AudioComponent.Play` (`self.11L-clock_ticking-49566274_Cue`) 0.0)
      (`self.Slow Time`))))

(event `Destroyer`
  (`AudioComponent.Stop` (`self.11L-clock_ticking-49566274_Cue`))
  (`self.K2_DestroyActor`)
  (`self.Resume Time`))

(fn `Resume Time`
  (`GameplayStatics.SetGlobalTimeDilation` 1.0))

(fn `Slow Time`
  (`GameplayStatics.SetGlobalTimeDilation` (`self.SlowFactor`)))

(fn `UserConstructionScript`)