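; VR pawn component that runs a time-slow ability with a depletable meter.
; Tick drains TimeSlowProgress while IsTriggered and refills it otherwise, with no clamp here.
; TimeSlowStart, when meter remains, plays a whoosh and spawns a TimeSlowZone using capsule forward X/Y and camera height; TimeSlowEnd calls the zone's Destroyer.
; Separate SlowTime and ResumeTime functions set and reset global time dilation, uncalled within this component.
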(event `self.ReceiveTick`
  (params (DeltaSeconds :type "Float (single-precision)"))
  (if (`self.IsTriggered`)
    (set `self.TimeSlowProgress` (- (`self.TimeSlowProgress`) (* (`self.Multiplier`) DeltaSeconds)))
    (else
      (set `self.TimeSlowProgress` (+ (`self.TimeSlowProgress`) (* DeltaSeconds (`self.Multiplier`)))))))

(event `self.ReceiveBeginPlay`
  (bind _asvrpawn (cast `/Game/Blueprints/VRPawn` (`self.GetOwner`)))
  (set `self.Player` _asvrpawn))

(event `TimeSlowStart`
  (bind _player (`self.Player`))
  (bind (_returnvalue_x _returnvalue_y) (`KismetMathLibrary.BreakVector` (`SceneComponent.GetForwardVector` (`Character.CapsuleComponent` _player))))
  (bind (_returnvalue_x_2 _returnvalue_y_2 _returnvalue_z) (`KismetMathLibrary.BreakVector` (`SceneComponent.K2_GetComponentLocation` (`/Game/Blueprints/VRPawn.Camera` _player))))
  (if (> (`self.TimeSlowProgress`) 0.0)
    (`GameplayStatics.SpawnSoundAtLocation` "/Game/Blueprints/YX_SoundEffect/whoosh-fast-bright-vadi-sound-1-00-01.whoosh-fast-bright-vadi-sound-1-00-01" (`SceneComponent.K2_GetComponentLocation` (`Character.CapsuleComponent` (`self.Player`))) (struct) 1.0 1.0 0.0 null null)
    (bind _returnvalue (`|SpawnActorFromClass` "/Game/Blueprints/TimeSlow/TimeSlowZone.TimeSlowZone_C" (`KismetMathLibrary.Conv_VectorToTransform` (`KismetMathLibrary.MakeVector` _returnvalue_x _returnvalue_y _returnvalue_z)) "Undefined" "MultiplyWithRoot" null null))
    (set `self.Zone` _returnvalue)))

(event `TimeSlowEnd`
  (`/Game/Blueprints/TimeSlow/TimeSlowZone.Destroyer` (`self.Zone`)))

(fn `ResumeTime`
  (`GameplayStatics.SetGlobalTimeDilation` 1.0))

(fn `SlowTime`
  (`GameplayStatics.SetGlobalTimeDilation` (`self.SlowFactor`)))