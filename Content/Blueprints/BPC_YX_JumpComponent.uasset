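; Actor component that gives a VR pawn a physical jump triggered by raising both hands.
; BeginPlay adds jump, land and grunt audio components through the Player reference, which is only assigned later in YXJump.
; When jumping mode allows, YXJump plays sounds, samples both grip heights across a brief delay, and jumps if both rise fast enough.
; Landing sound and finished flag follow immediately if grounded or the gesture fails, without awaiting touchdown.
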(event `self.ReceiveBeginPlay`
  (bind _returnvalue (`|AddComponentByClass` :`self` (`self.Player`) :`Class` "/Script/Engine.AudioComponent"))
  (`AudioComponent.SetSound` _returnvalue "/Game/Blueprints/YX_SoundEffect/Jump_Cue.Jump_Cue")
  (set `self.PlayerJumpAudio` _returnvalue)
  (bind _returnvalue_2 (`|AddComponentByClass` :`self` (`self.Player`) :`Class` "/Script/Engine.AudioComponent"))
  (`AudioComponent.SetSound` _returnvalue_2 "/Game/Blueprints/YX_SoundEffect/Land_Cue.Land_Cue")
  (set `self.PlayerLandAudio` _returnvalue_2)
  (bind _returnvalue_3 (`|AddComponentByClass` :`self` (`self.Player`) :`Class` "/Script/Engine.AudioComponent"))
  (`AudioComponent.SetSound` _returnvalue_3 "/Game/Blueprints/YX_SoundEffect/MaleGrunt_Cue.MaleGrunt_Cue")
  (set `self.PlayerGruntAudio` _returnvalue_3))

(event `YXJump`
  (bind _player (`self.Player`))
  (bind (_rightdifference_x _rightdifference_y _rightdifference_z) (`KismetMathLibrary.BreakVector` (`self.RightDifference`)))
  (bind (_leftdifference_x _leftdifference_y _leftdifference_z) (`KismetMathLibrary.BreakVector` (`self.LeftDifference`)))
  (bind _player_2 (`self.Player`))
  (bind _player_3 (`self.Player`))
  (bind _player_4 (`self.Player`))
  (bind _asvrpawn (cast `/Game/Blueprints/VRPawn` (`self.GetOwner`)))
  (set `self.Player` _asvrpawn)
  (if (`/Game/Blueprints/VRPawn.IsJumpingMode` _player)
    (if (`/Game/Blueprints/VRPawn.IsJumpingFinished` _player)
      (`AudioComponent.Play` (`self.PlayerJumpAudio`) 0.0)
      (`AudioComponent.Play` (`self.PlayerGruntAudio`) 0.0)
      (set `/Game/Blueprints/VRPawn.IsJumpingFinished` false _player_4)
      (set `self.PrevRightHandPos` (`SceneComponent.K2_GetComponentLocation` (`/Game/Blueprints/VRPawn.MotionControllerRightGrip` _player_4)))
      (set `self.PrevLeftHandPos` (`SceneComponent.K2_GetComponentLocation` (`/Game/Blueprints/VRPawn.MotionControllerLeftGrip` _player_4)))
      (`KismetSystemLibrary.Delay` 0.01)
      (set `self.RightDifference` (- (`SceneComponent.K2_GetComponentLocation` (`/Game/Blueprints/VRPawn.MotionControllerRightGrip` _player_3)) (`self.PrevRightHandPos`)))
      (set `self.LeftDifference` (- (`SceneComponent.K2_GetComponentLocation` (`/Game/Blueprints/VRPawn.MotionControllerLeftGrip` _player_3)) (`self.PrevLeftHandPos`)))
      (if (and (>= _leftdifference_z 1.5) (>= _rightdifference_z 1.5))
        (cast `Character` (`self.GetOwner`))
        (`Character.Jump` _player_2)
        (bind _ismovingonground (`/Game/Blueprints/VRPawn.IsCharacterMovingOnGround` (`self.Player`)))
        (if _ismovingonground
          (set `/Game/Blueprints/VRPawn.IsJumpingFinished` true _player_2 :!label _label)
          (`AudioComponent.Play` (`self.PlayerLandAudio`) 0.0))
        (else
          (goto _label))))))